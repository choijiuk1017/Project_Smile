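; A scene capture actor, labeled a mirror in its debug prints, that works only while the player is nearby.
; A box overlap by the player pawn enables capture component and actor ticking, which is off at BeginPlay.
; Each tick rotates the capture component to face the player pawn.
; Leaving the box stops actor tick and disables SceneComponent tick, leaving the capture component's tick enabled.
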(event OnComponentBeginOverlap(Box)
  (params (OverlappedComponent :type Primitive%20Component%20Object%20Reference) (OtherActor :type Actor%20Object%20Reference) (OtherComp :type Primitive%20Component%20Object%20Reference) (OtherBodyIndex :type Integer) (bFromSweep :type Boolean) (SweepResult :type Hit%20Result%20Structure%20%28by%20ref%29))
  (Development|PrintString "거울 시작")
  (if (== OtherActor (Game|Player|GetPlayerPawn 0))
    (Components|Tick|SetComponentTickEnabled (Variables|DecalActor|GetCaptureComponent2D) true)
    (Actor|Tick|SetActorTickEnabled true)))

(event OnComponentEndOverlap(Box)
  (params (OverlappedComponent :type Primitive%20Component%20Object%20Reference) (OtherActor :type Actor%20Object%20Reference) (OtherComp :type Primitive%20Component%20Object%20Reference) (OtherBodyIndex :type Integer))
  (Development|PrintString "거울 종료")
  (if (== OtherActor (Game|Player|GetPlayerPawn 0))
    (Components|Tick|SetComponentTickEnabled (Variables|Default|GetSceneComponent) false)
    (Actor|Tick|SetActorTickEnabled false)))

(event EventBeginPlay
  (Actor|Tick|SetActorTickEnabled false))

(event EventTick
  (params (DeltaSeconds :type Float%20%28single-precision%29))
  (Transformation|SetWorldRotation (Variables|DecalActor|GetCaptureComponent2D) (Math|Rotator|FindLookatRotation (Transformation|GetWorldLocation (Variables|DecalActor|GetCaptureComponent2D)) (Transformation|GetActorLocation (Game|Player|GetPlayerPawn 0))) false false))

(fn ConstructionScript)